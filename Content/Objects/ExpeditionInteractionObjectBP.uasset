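; Clickable expedition object, currently hard-coded as a wood chest, that the party can interact with.
; BeginPlay loads its data and sprite texture from GameInstance containers and binds left-click on a child DynamicPaperSpriteActor.
; Clicks work at any distance in rooms, otherwise only within a facing-dependent Y band, opening a side-placed widget and locking party movement and turning.
; SetObjectStyle swaps textures, applying "Unused" when IsUsed is true and "Used" when false.
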(event Custom|OnClicked_Event
  (params (TouchedActor :type Actor%20Object%20Reference) (ButtonPressed :type Key%20Structure :default "None"))
  (if (== ButtonPressed "LeftMouseButton")
    (bind _asbpgame_instance (Utilities|Casting|CastToBPGameInstance (Game|GetGameInstance)))
    (if (not (Variables|/Game/BPGameInstance.BPGameInstance_C|GetInteractionWithObjectIsPerformed _asbpgame_instance))
      ;[1 1 1] Если пати в комнате, то объект прожимается на любом расстоянии до него
      (bind _asbpgame_instance_2 (Utilities|Casting|CastToBPGameInstance (Game|GetGameInstance)))
      (CallFunction|InteractwithObject (Variables|/Game/BPGameInstance.BPGameInstance_C|GetPartyInTheRoom _asbpgame_instance_2)))))

(event EventBeginPlay
  (bind _returnvalue (Game|ConstructObjectfromClass "/Script/RoguelikeThing.LogPrinter" self))
  (Variables|Default|SetLogPrinter _returnvalue)
  (CallFunction|InitObjectData "Default" "Container" "Common" "WoodChest")
  (bind _asbpgame_instance (Utilities|Casting|CastToBPGameInstance (Game|GetGameInstance)))
  (bind _returnvalue_2 (Class|TextureContainer|FindTexture (Variables|/Game/BPGameInstance.BPGameInstance_C|GetExpeditionInteractionObjectsTextureContainer _asbpgame_instance) "Default" "Container" "Common" "WoodChest" "Unused"))
  (bind _asdynamic_paper_sprite_actor (Utilities|Casting|CastToDynamicPaperSpriteActor (Variables|/Script/Engine.ChildActorComponent|GetChildActor (Variables|Default|GetObjectSprite))))
  (Rendering|Material|SetMaterial (Variables|/Script/Paper2D.PaperSpriteActor|GetRenderComponent _asdynamic_paper_sprite_actor) 0 "/Game/Materials/SpriteMaterial.SpriteMaterial")
  (Class|DynamicPaperSpriteActor|SetTexture _asdynamic_paper_sprite_actor _returnvalue_2 "Bottom_Center")
  (EventDispatchers|AssignOnClicked _asdynamic_paper_sprite_actor (delegate Custom|OnClicked_Event)))

(event Collision|EventActorBeginOverlap
  (params (OtherActor :type Actor%20Object%20Reference)))

(event EventTick
  (params (DeltaSeconds :type Float%20%28single-precision%29)))

(fn ConstructionScript)

(fn InteractwithObject
  (params (InteractWithoutRegardToDistance :type Boolean))
  (bind _self self)
  (bind _self_2 self)
  (bind _returnvalue (Transformation|GetActorLocation _self))
  (bind _returnvalue_2 (Transformation|GetActorLocation _self_2))
  (if InteractWithoutRegardToDistance
    (bind _returnvalue_3 (UserInterface|CreateWidget "/Game/UI/Widgets/ExpeditionObjectInteraction/ExpeditionObjectInteractionWidget.ExpeditionObjectInteractionWidget_C" (Game|GetPlayerController 0) :!label _label))
    ;[1 1 1] Созданный виджет взаимодействия с объектом помещается на ту сторону, где он не будет загораживать пати, в зависимости от направления её взгляда
    (bind _asparty (Utilities|Casting|CastToParty (Game|Player|GetPlayerPawn 0)))
    (Default|SetLocationSide _returnvalue_3 (Variables|/Game/Objects/Party.Party_C|GetLookingRight _asparty))
    (bind _asbpgame_instance (Utilities|Casting|CastToBPGameInstance (Game|GetGameInstance)))
    (Variables|/Game/BPGameInstance.BPGameInstance_C|SetInteractionWithObjectIsPerformed _asbpgame_instance true)
    ;[1 1 1] Пока пати взаимодействует с объектом, оно не может ходить
    (bind _asparty_2 (Utilities|Casting|CastToParty (Game|Player|GetPlayerPawn 0)))
    (Variables|/Game/Objects/Party.Party_C|SetMovementAllowed _asparty_2 false)
    (Variables|/Game/Objects/Party.Party_C|SetTurnentAllowed _asparty_2 false)
    (Default|ExpeditionInteractionObjectDataInit _returnvalue_3 (Variables|Default|GetExpeditionInteractionObjectData) self)
    (UserInterface|Viewport|AddtoViewport _returnvalue_3 0)
    (else
      ;[1 1 1] Если переменная InteractWithoutRegardToDistance говорит о том, что взаимодействие с объектом можнет происходить только при приближении к нему пати, то степень этого приближения вычисляется здесь, при чём с учётом направления взгляда пати.
      (bind _asparty_3 (Utilities|Casting|CastToParty (Game|Player|GetPlayerPawn 0)))
      (if (Variables|/Game/Objects/Party.Party_C|GetLookingRight _asparty_3)
        (if (and (< (.y (Transformation|GetActorLocation _asparty_3)) (- (.y _returnvalue_2) 2.5e+02)) (> (.y (Transformation|GetActorLocation _asparty_3)) (- (.y _returnvalue_2) 7.5e+02)))
          (goto _label))
        (elif (and (< (+ (.y _returnvalue) 2.5e+02) (.y (Transformation|GetActorLocation _asparty_3))) (> (+ (.y _returnvalue) 7.5e+02) (.y (Transformation|GetActorLocation _asparty_3))))
          (goto _label))))))

(fn InitObjectData
  (params (ModuleName :type String) (CategoryName :type String) (SubCategoryName :type String) (ObjectId :type String))
  (bind _asbpgame_instance (Utilities|Casting|CastToBPGameInstance (Game|GetGameInstance)))
  (bind _returnvalue (Class|ExpeditionInteractionObjectContainer|FindData (Variables|/Game/BPGameInstance.BPGameInstance_C|GetInteraction%20Objects%20Data%20Array _asbpgame_instance) ModuleName CategoryName SubCategoryName ObjectId))
  (if (Utilities|IsValid _returnvalue)
    (Variables|Default|SetExpeditionInteractionObjectData _returnvalue)
    (else
      (Class|LogPrinter|PrintLog (Variables|Default|GetLogPrinter) (Utilities|String|Append "!!! An error occurred in the ExpeditionInteractionObjectBP class in the BP_InitObjectData function - The object with  id \"" ObjectId "\" was not found in the list of all expedition interaction objects.") "ERROR"))))

(fn SetObjectStyle
  (params (IsUsed :type Boolean))
  (bind _asbpgame_instance (Utilities|Casting|CastToBPGameInstance (Game|GetGameInstance)))
  (bind _asdynamic_paper_sprite_actor (Utilities|Casting|CastToDynamicPaperSpriteActor (Variables|/Script/Engine.ChildActorComponent|GetChildActor (Variables|Default|GetObjectSprite))))
  (if IsUsed
    (bind _returnvalue (Class|TextureContainer|FindTexture (Variables|/Game/BPGameInstance.BPGameInstance_C|GetExpeditionInteractionObjectsTextureContainer _asbpgame_instance) "Default" "Container" "Common" "WoodChest" "Unused"))
    (Class|DynamicPaperSpriteActor|SetTexture _asdynamic_paper_sprite_actor _returnvalue "Bottom_Center")
    (Variables|Default|SetIsUsed true)
    (else
      (bind _returnvalue_2 (Class|TextureContainer|FindTexture (Variables|/Game/BPGameInstance.BPGameInstance_C|GetExpeditionInteractionObjectsTextureContainer _asbpgame_instance) "Default" "Container" "Common" "WoodChest" "Used"))
      (Class|DynamicPaperSpriteActor|SetTexture _asdynamic_paper_sprite_actor _returnvalue_2 "Bottom_Center")
      (Variables|Default|SetIsUsed false))))